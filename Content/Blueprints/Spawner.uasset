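; Spawner actor that periodically spawns a random actor from its Spawnables list in a ring around itself.
; Tick accumulates a timer and, on reaching SpawnTime, resets it and spawns at a time-driven sine/cosine offset with random radius per axis, at world Z zero.
; Each spawned actor is then yawed toward the player pawn, with a 90-degree offset.
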(event `self.ReceiveTick`
  (params (DeltaSeconds :type "Float (single-precision)"))
  (bind _timer (`self.Timer`))
  (bind _returnvalue (* (`GameplayStatics.GetTimeSeconds`) 1000.0))
  (set `self.Timer` (+ _timer DeltaSeconds))
  (if (>= _timer (`self.SpawnTime`))
    (set `self.Timer` 0.0)
    (bind _returnvalue_2 (`|SpawnActorFromClass` (`|GetArrayItem` (`self.Spawnables`) (`KismetMathLibrary.RandomInteger` (`KismetArrayLibrary.Array_Length` (`self.Spawnables`)))) (`KismetMathLibrary.Conv_VectorToTransform` (`KismetMathLibrary.MakeVector` (+ (.x (`self.K2_GetActorLocation`)) (* (`KismetMathLibrary.DegSin` _returnvalue) (`KismetMathLibrary.RandomFloatInRange` 300.0 600.0))) (+ (.y (`self.K2_GetActorLocation`)) (* (`KismetMathLibrary.DegCos` _returnvalue) (`KismetMathLibrary.RandomFloatInRange` 300.0 600.0))))) "Undefined" "OverrideRootScale" null null))
    (`self.K2_SetActorRotation` _returnvalue_2 (`KismetMathLibrary.MakeRotator` 0.0 0.0 (+ (.yaw (`KismetMathLibrary.FindLookAtRotation` (.location (`self.GetTransform` _returnvalue_2)) (`self.K2_GetActorLocation` (`GameplayStatics.GetPlayerPawn` 0)))) -90.0)) false)))

(fn `UserConstructionScript`)