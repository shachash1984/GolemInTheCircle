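; GearVR_Pawn is a VR pawn for Gear VR that detects touchpad gestures and shows the result on a text component.
; On BeginPlay it sets an eye-level tracking origin and offsets the VR camera root to a configured height.
; Touch press and release positions are compared on release: short movement counts as a tap, otherwise the dominant axis and sign classify a left, right, up or down swipe.
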(event `InputTouch`
  (params (Location :type "Vector Structure") (FingerIndex :type "ETouchIndex Enum"))
  (bind (_locationx _locationy) (`PlayerController.GetInputTouchState` (`GameplayStatics.GetPlayerController` 0) "Touch1"))
  (bind _returnvalue (- (`self.TouchStart`) (`self.TouchEnd`)))
  (bind _returnvalue_2 (`KismetMathLibrary.MakeVector2D` _locationx _locationy))
  (bind (_x _y) (`KismetMathLibrary.BreakVector2D` _returnvalue))
  (:`Pressed`
    (set `self.TouchStart` _returnvalue_2))
  (:`Released`
    (set `self.TouchEnd` _returnvalue_2)
    (if (> (`KismetMathLibrary.VSize2D` _returnvalue) 20.0)
      (if (> (`KismetMathLibrary.Abs` _x) (`KismetMathLibrary.Abs` _y))
        (if (< _x 0.0)
          ;[1 1 1] Swipe Left
          (`TextRenderComponent.K2_SetText` (`self.PlayerText`) (`self.SwipeLeft`))
          (else
            ;[1 1 1] Swipe Right
            (`TextRenderComponent.K2_SetText` (`self.PlayerText`) (`self.SwipeRight`))))
        (elif (> _y 1.0)
          ;[1 1 1] Swipe Up
          (`TextRenderComponent.K2_SetText` (`self.PlayerText`) (`self.SwipeUp`))
          (else
            ;[1 1 1] Swipe Down
            (`TextRenderComponent.K2_SetText` (`self.PlayerText`) (`self.SwipeDown`)))))
      (else
        ;[1 1 1] Single Tap
        (`TextRenderComponent.K2_SetText` (`self.PlayerText`) (`self.TouchTap`))))))

(event `self.ReceiveBeginPlay`
  (`HeadMountedDisplayFunctionLibrary.SetTrackingOrigin` "Eye")
  (`SceneComponent.K2_SetRelativeLocation` (`self.VRCameraRoot`) (`self.CameraHeight`) false false))

(fn `UserConstructionScript`)